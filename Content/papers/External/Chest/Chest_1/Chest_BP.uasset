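; Interactable chest Blueprint whose lid opens and closes when the player presses the interaction key inside its trigger box.
; Box overlap enables input from the first player controller and sets a flag; leaving clears it, disables input and reverses the timeline to close the lid.
; Each press alternates through a FlipFlop between playing and reversing a timeline that drives the pitch of the lid mesh's relative rotation.
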(event OnComponentEndOverlap(Box)
  (params (OverlappedComponent :type Primitive%20Component%20Object%20Reference) (OtherActor :type Actor%20Object%20Reference) (OtherComp :type Primitive%20Component%20Object%20Reference) (OtherBodyIndex :type Integer))
  (Variables|Default|SetBegin_overlap false)
  (Input|DisableInput (Game|GetPlayerController 0))
  (bind _rotation (Timeline|Open_cest Reverse)
    (:Update
      (Transformation|SetRelativeRotation (Variables|Default|GetChest_1_iron_1_001) (Math|Rotator|MakeRotator 0.0 _rotation 0.0) false false))))

(event OnComponentBeginOverlap(Box)
  (params (OverlappedComponent :type Primitive%20Component%20Object%20Reference) (OtherActor :type Actor%20Object%20Reference) (OtherComp :type Primitive%20Component%20Object%20Reference) (OtherBodyIndex :type Integer) (bFromSweep :type Boolean) (SweepResult :type Hit%20Result%20Structure%20%28by%20ref%29))
  (Input|EnableInput (Game|GetPlayerController 0))
  (Variables|Default|SetBegin_overlap true))

(event Input|ActionEvents|InputActionIteractions
  (params (Key :type Key%20Structure :default "AnyKey"))
  (:Pressed
    (if (Variables|Default|GetBegin_overlap)
      (Utilities|FlowControl|FlipFlop
        (:A
          (bind _rotation (Timeline|Open_cest Play)
            (:Update
              (Transformation|SetRelativeRotation (Variables|Default|GetChest_1_iron_1_001) (Math|Rotator|MakeRotator 0.0 _rotation 0.0) false false))))
        (:B
          (Timeline|Open_cest Reverse))))))

(fn ConstructionScript)